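; BP_Platform is a moving platform actor that starts its motion automatically on BeginPlay.
; It first shifts the whole actor by a fixed offset along world X, then plays a Timeline.
; Each Timeline update sets the world location of the SMIntersectionFloor component by lerping between the actor's current location and that location plus the Distance vector.
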(event EventBeginPlay
  (Transformation|SetActorLocation (+ (Transformation|GetActorLocation) "180.000000,0.000000,0.000000") false false)
  (bind _newtrack_0 (Timeline|Timeline Play)
    (:Update
      (Transformation|SetWorldLocation (Variables|Default|GetSM_Intersection_Floor) (Math|Vector|Lerp(Vector) (Transformation|GetActorLocation) (+ (Transformation|GetActorLocation) (Variables|Default|GetDistance)) _newtrack_0) false false))))

(event Collision|EventActorBeginOverlap
  (params (OtherActor :type Actor%20Object%20Reference)))

(event EventTick
  (params (DeltaSeconds :type Float%20%28single-precision%29)))

(fn ConstructionScript)