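; BP_JetToggle is a thruster hazard that burns the third-person character while it stands in the exhaust.
; BeginPlay spawns a blue rocket exhaust Niagara system and plays a fire sound at the Arrow's transform.
; Capsule overlap applies damage immediately, then repeats it on a looping timer until the overlap ends.
; RecieverFunction shuts the jet off by deactivating the effect and destroying the capsule, with no path to re-enable it.
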(event OnComponentBeginOverlap(Capsule)
  (params (OverlappedComponent :type Primitive%20Component%20Object%20Reference) (OtherActor :type Actor%20Object%20Reference) (OtherComp :type Primitive%20Component%20Object%20Reference) (OtherBodyIndex :type Integer) (bFromSweep :type Boolean) (SweepResult :type Hit%20Result%20Structure%20%28by%20ref%29))
  (bind _asbp_third_person_character (Utilities|Casting|CastToBP_ThirdPersonCharacter OtherActor))
  (CallFunction|DOT)
  (CallFunction|StartDOT))

(event OnComponentEndOverlap(Capsule)
  (params (OverlappedComponent :type Primitive%20Component%20Object%20Reference) (OtherActor :type Actor%20Object%20Reference) (OtherComp :type Primitive%20Component%20Object%20Reference) (OtherBodyIndex :type Integer))
  (Utilities|Casting|CastToBP_ThirdPersonCharacter OtherActor)
  (CallFunction|EndDOT))

(event Custom|StartDOT
  (bind _returnvalue (Utilities|Time|SetTimerbyEvent (delegate Custom|DOT) 0.3 true))
  (Variables|Default|SetDOTTimer _returnvalue))

(event Custom|DOT
  (Game|Damage|ApplyDamage (stale OnComponentBeginOverlap(Capsule) _asbp_third_person_character) 1e+01 0 0))

(event Custom|EndDOT
  (Utilities|Time|ClearandInvalidateTimerbyHandle (Variables|Default|GetDOTTimer)))

(event EventBeginPlay
  (bind _arrow (Variables|Default|GetArrow))
  (bind _returnvalue (Transformation|GetWorldTransform _arrow))
  (Game|SpawnActorfromClass "/Script/Niagara.NiagaraActor" (Math|Transform|MakeTransform (.location _returnvalue) (.rotation _returnvalue) (.scale _returnvalue)) "Undefined" "MultiplyWithRoot" 0 0)
  (bind _returnvalue_2 (Niagara|SpawnSystematLocation "/Game/RocketThrusterExhaustFX/FX/NS_RocketExhaust_Blue.NS_RocketExhaust_Blue" (.location _returnvalue) (.rotation _returnvalue) (.scale _returnvalue) false))
  (Audio|PlaySoundatLocation "/Game/StarterContent/Audio/Fire01.Fire01" (.location _returnvalue) "0, 0, 0" 1.0 1.0 0.0 0 0 0 0))

(event EventRecieverFunction
  (params (Group :type Integer))
  (Components|Activation|Deactivate (stale EventBeginPlay _returnvalue_2))
  (Components|DestroyComponent (Variables|Default|GetCapsule)))

(fn ConstructionScript)